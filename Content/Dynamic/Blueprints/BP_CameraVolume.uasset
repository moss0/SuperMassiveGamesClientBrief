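; BP_CameraVolume is a trigger volume that gives the game's BP_Camera a target position when overlapped.
; At BeginPlay it caches the player character and finds the camera actor in the level.
; Box overlap, checked against the player via IsPlayer, registers the volume as current and sends the CameraTarget location plus a vertical offset.
; End overlap only clears the overlapping flag, leaving the camera's volume and target unchanged.
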(event OnComponentEndOverlap(Box)
  (params (OverlappedComponent :type Primitive%20Component%20Object%20Reference) (OtherActor :type Actor%20Object%20Reference) (OtherComp :type Primitive%20Component%20Object%20Reference) (OtherBodyIndex :type Integer))
  (CallFunction|IsPlayer OtherActor)
  (Variables|Default|SetisOverlapping false))

(event OnComponentBeginOverlap(Box)
  (params (OverlappedComponent :type Primitive%20Component%20Object%20Reference) (OtherActor :type Actor%20Object%20Reference) (OtherComp :type Primitive%20Component%20Object%20Reference) (OtherBodyIndex :type Integer) (bFromSweep :type Boolean) (SweepResult :type Hit%20Result%20Structure%20%28by%20ref%29))
  (CallFunction|IsPlayer OtherActor)
  (Variables|Default|SetisOverlapping true)
  (Variables|/Game/Dynamic/Blueprints/BP_Camera.BP_Camera_C|SetcurrVol (Variables|Default|Getcamera) self)
  (Variables|/Game/Dynamic/Blueprints/BP_Camera.BP_Camera_C|SettargetPos (Variables|Default|Getcamera) (+ (Transformation|GetWorldLocation (Variables|Default|GetCameraTarget)) (Math|Vector|MakeVector 0.0 0.0 (Variables|Default|GetverticalOffset)))))

(event EventBeginPlay
  (Variables|Default|Setplayer (Game|GetPlayerCharacter 0))
  (bind _returnvalue (Actor|GetActorOfClass "/Game/Dynamic/Blueprints/BP_Camera.BP_Camera_C"))
  (Variables|Default|Setcamera _returnvalue))

(fn ConstructionScript)

(fn IsPlayer
  (params (A :type Object%20Object%20Reference))
  (if (== A (Variables|Default|Getplayer))
    _))
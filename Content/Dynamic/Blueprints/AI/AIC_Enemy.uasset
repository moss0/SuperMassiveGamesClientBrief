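; AI controller for enemies that switches between patrolling and hunting based on what it perceives.
; On possess, after a short delay, it runs BT_Enemy, stores the player as the Blackboard target and starts patrolling.
; Perception updates check each actor's stimuli by sense class; sight sets the Blackboard state enum to hunting, otherwise patrolling.
; Hearing is checked but triggers nothing, and HandleSensedSight is empty.
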(event OnPerceptionUpdated(AIPerception)
  (params (UpdatedActors :type Array%20of%20Actor%20Object%20References))
  (for _array_element UpdatedActors
    (Utilities|FlowControl|Sequence
      (:then_0
        (bind _sensed (CallFunction|CanSenseActor _array_element "NewEnumerator1"))
        (if _sensed
          (CallFunction|SetStateasHunting)
          (else
            (CallFunction|SetStateasPatrolling))))
      (:then_1
        (bind _sensed_2 (CallFunction|CanSenseActor _array_element "NewEnumerator2"))
        (if _sensed_2
          _)))))

(event EventPossess
  (params (PossessedPawn :type Pawn%20Object%20Reference))
  (Utilities|FlowControl|Delay 0.2)
  (AI|RunBehaviorTree "/Game/Dynamic/Blueprints/AI/BT_Enemy.BT_Enemy")
  (AI|Components|Blackboard|SetValueasObject (Variables|Default|GetBlackboard) (Variables|Default|GettargetActorKeyName) (Game|GetPlayerCharacter 0))
  (CallFunction|SetStateasPatrolling))

(fn ConstructionScript)

(fn SetStateasPatrolling
  (AI|Components|Blackboard|SetValueasEnum (Variables|Default|GetBlackboard) (Variables|Default|GetstateKeyName) (Utilities|Enum|LiteralenumE_EnemyStates "NewEnumerator1")))

(fn SetStateasHunting
  (AI|Components|Blackboard|SetValueasEnum (Variables|Default|GetBlackboard) (Variables|Default|GetstateKeyName) (Utilities|Enum|LiteralenumE_EnemyStates "NewEnumerator0")))

(fn HandleSensedSight)

(fn CanSenseActor
  (params (Actor :type Actor%20Object%20Reference) (Sense :type E_AISense%20Enum :default "NewEnumerator0"))
  (bind _info (Class|AIPerceptionComponent|GetActorsPerception (Variables|Default|GetAIPerception) Actor))
  (for _array_element (.LastSensedStimuli (Utilities|Struct|BreakActorPerceptionBlueprintInfo _info))
    (bind _returnvalue (Class|AIPerceptionSystem|GetSenseClassforStimulus _array_element))
    (if (== _returnvalue (Utilities|Select :Index Sense :NewEnumerator0 0 :NewEnumerator1 "/Script/AIModule.AISense_Sight" :NewEnumerator2 "/Script/AIModule.AISense_Hearing"))
      (return (.bSuccessfullySensed (Utilities|Struct|BreakAIStimulus _array_element)) _array_element))))
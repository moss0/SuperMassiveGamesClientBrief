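; Camera actor that becomes the player's view target on BeginPlay and focuses on the player character.
; Each Tick, a rotate mode aims it at the focus rigidly or smoothly, then a move mode positions it.
; Fixed mode eases toward a target position plus vertical offset, at a room-change speed; follow mode snaps only Z to the focus.
; MoveToFocusWithOffset is defined but never called.
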(event EventBeginPlay
  (bind _returnvalue (Game|GetPlayerCharacter 0))
  (Utilities|FlowControl|Sequence
    (:then_0
      (Game|Player|SetViewTargetwithBlend (Game|GetPlayerController 0) self 0.0 "VTBlend_Linear" 0.0 false))
    (:then_1
      (Utilities|IsValid _returnvalue
        (:Is%20Valid
          (Variables|Default|Setplayer _returnvalue))))
    (:then_2
      (Variables|Default|SettargetPos (Transformation|GetActorLocation)))
    (:then_3
      (Variables|Default|Setfocus (Variables|Default|Getplayer)))))

(event EventTick
  (params (DeltaSeconds :type Float%20%28single-precision%29))
  (Variables|Default|SetDelta%20Seconds DeltaSeconds)
  (Utilities|FlowControl|Sequence
    (:then_0
      (switch Utilities|FlowControl|Switch|SwitchonEnum_CameraRotationModes (Variables|Default|GetcameraRotateMode)
        (:NewEnumerator1
          (bind _rotation (CallFunction|RotatetoFocus))
          (Transformation|SetActorRotation _rotation))
        (:NewEnumerator0
          (bind _rotation_2 (CallFunction|InterpRotatetoFocus))
          (Transformation|SetActorRotation _rotation_2))))
    (:then_1
      (switch Utilities|FlowControl|Switch|SwitchonEnum_CameraTranslateModes (Variables|Default|GetcameraMoveMode)
        (:NewEnumerator0
          (CallFunction|InterptoTargetPos))
        (:NewEnumerator1
          (CallFunction|MovetoFocusZPos))))))

(fn ConstructionScript)

(fn RotatetoFocus
  (return (Math|Rotator|FindLookatRotation (Transformation|GetActorLocation) (Transformation|GetActorLocation (Variables|Default|Getfocus)))))

(fn InterpRotatetoFocus
  (return (Math|Interpolation|RInterpTo (.rotation (Transformation|GetActorTransform)) (Math|Rotator|FindLookatRotation (Transformation|GetActorLocation) (Transformation|GetActorLocation (Variables|Default|Getfocus))) (Variables|Default|GetDelta%20Seconds) (Variables|Default|GetrotateInterpSpeed))))

(fn InterptoTargetPos
  (bind _returnvalue (Transformation|GetActorLocation))
  (if (not (Utilities|Operators|EqualEqual (Variables|Default|GettargetPos) _returnvalue 0.0))
    (Transformation|SetActorLocation (Math|Interpolation|VInterpTo _returnvalue (+ (Variables|Default|GettargetPos) (Math|Vector|MakeVector 0.0 0.0 (Variables|Default|GetVerticalOffsetFromTargetPos))) (Variables|Default|GetDelta%20Seconds) (Variables|Default|GetroomChangeInterpSpeed)) false false)
    (return)))

(fn MovetoFocusZPos
  (bind _returnvalue (Transformation|GetActorLocation))
  (bind _focus (Variables|Default|Getfocus))
  (bind _returnvalue_2 (Transformation|GetActorLocation _focus))
  (if (not (== (.z _returnvalue) (.z _returnvalue_2)))
    (LocalVariables|SetcameraX (.x _returnvalue))
    (LocalVariables|SetcameraY (.y _returnvalue))
    (LocalVariables|SetfocusZ (.z _returnvalue_2))
    (bind _output_get (LocalVariables|Setvector (Math|Vector|MakeVector (LocalVariables|GetcameraX) (LocalVariables|GetcameraY) (LocalVariables|GetfocusZ))))
    (Transformation|SetActorLocation _output_get false false)))

(fn MovetoFocuswithOffset
  (Transformation|SetActorLocation (+ (Transformation|GetActorLocation (Variables|Default|Getfocus)) (Variables|Default|GetcameraTargetOffset)) false false))
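; Enemy AI pawn that chases pawns it sees and prints a catch message when its box overlaps the player character.
; PawnSensing starts a move toward the seen pawn, while a retriggerable one-second delay halts it at its current location once sightings stop.
; It also caches the BP_Camera actor on BeginPlay and provides a debug-drawn downward line trace helper, neither used in these graphs.
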(event OnSeePawn(PawnSensing)
  (params (Pawn :type Pawn%20Object%20Reference))
  (bind _self self)
  (Utilities|FlowControl|Sequence
    (:then_0
      (AI|AIMoveTo self "0, 0, 0" Pawn 5.0 false))
    (:then_1
      (Utilities|FlowControl|RetriggerableDelay 1.0)
      (AI|AIMoveTo _self (Transformation|GetActorLocation _self) 0 5.0 false))))

(event OnComponentBeginOverlap(Box)
  (params (OverlappedComponent :type Primitive%20Component%20Object%20Reference) (OtherActor :type Actor%20Object%20Reference) (OtherComp :type Primitive%20Component%20Object%20Reference) (OtherBodyIndex :type Integer) (bFromSweep :type Boolean) (SweepResult :type Hit%20Result%20Structure%20%28by%20ref%29))
  (if (== OtherActor (Game|GetPlayerCharacter 0))
    (Development|PrintString "Got you")))

(event EventBeginPlay
  ;[0.05098 0.05098 0.05098] BeginPlay
  (Utilities|FlowControl|Sequence
    (:then_0
      (bind _returnvalue (Actor|GetActorOfClass "/Game/Dynamic/Blueprints/BP_Camera.BP_Camera_C"))
      (Utilities|IsValid _returnvalue
        (:Is%20Valid
          (Variables|Default|Setcamera _returnvalue))))))

(fn ConstructionScript)

(fn RaycastDownwards
  (bind _returnvalue (Transformation|GetActorLocation))
  (bind (_outhit _returnvalue_2) (Collision|LineTraceByChannel _returnvalue (+ _returnvalue (* (Math|Vector|GetUpVector (Transformation|GetActorRotation)) (Variables|Default|GetraycastDownSize) -1)) "TraceTypeQuery1" false 0 "ForOneFrame" true "(R=0.000000,G=0.897234,B=1.000000,A=1.000000)" "(R=1.000000,G=0.532573,B=0.000000,A=1.000000)" 1.0))
  (return _outhit _returnvalue_2))
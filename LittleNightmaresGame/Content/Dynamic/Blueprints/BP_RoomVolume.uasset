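; BP_RoomVolume is a room trigger that points BP_PlayerCamera at its own CameraTarget component when the player enters.
; Box overlap events track whether the player is inside and write the target's world location to the camera's TargetPos on entry.
; In the Camera Target Follow Player Zpos RoomState, Tick keeps updating TargetPos while overlapped and moves CameraTarget to the player's height, keeping its X and Y.
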(event OnComponentBeginOverlap(Box)
  (params (OverlappedComponent :type Primitive%20Component%20Object%20Reference) (OtherActor :type Actor%20Object%20Reference) (OtherComp :type Primitive%20Component%20Object%20Reference) (OtherBodyIndex :type Integer) (bFromSweep :type Boolean) (SweepResult :type Hit%20Result%20Structure%20%28by%20ref%29))
  (if (== OtherActor (Game|GetPlayerCharacter 0))
    (Variables|Default|SetisOverlapping true)
    (Variables|/Game/Dynamic/Blueprints/BP_PlayerCamera.BP_PlayerCamera_C|SettargetPos (Variables|Default|GetplayerCamera) (Transformation|GetWorldLocation (Variables|Default|GetCameraTarget)))))

(event OnComponentEndOverlap(Box)
  (params (OverlappedComponent :type Primitive%20Component%20Object%20Reference) (OtherActor :type Actor%20Object%20Reference) (OtherComp :type Primitive%20Component%20Object%20Reference) (OtherBodyIndex :type Integer))
  (if (== OtherActor (Game|GetPlayerCharacter 0))
    (Variables|Default|SetisOverlapping false)))

(event EventBeginPlay
  (Utilities|FlowControl|Sequence
    (:then_0
      (bind _returnvalue (Actor|GetActorOfClass "/Game/Dynamic/Blueprints/BP_PlayerCamera.BP_PlayerCamera_C"))
      (Utilities|IsValid _returnvalue
        (:Is%20Valid
          (Variables|Default|SetplayerCamera _returnvalue))))
    (:then_1
      (bind _returnvalue_2 (Actor|GetActorOfClass "/Game/Dynamic/Blueprints/BP_ThirdPersonCharacter.BP_ThirdPersonCharacter_C"))
      (Utilities|IsValid _returnvalue_2
        (:Is%20Valid
          (Variables|Default|Setplayer _returnvalue_2))))))

(event EventTick
  (params (DeltaSeconds :type Float%20%28single-precision%29))
  (switch Utilities|FlowControl|Switch|SwitchonEnum_RoomTypes (Variables|Default|GetroomState)
    (:NewEnumerator1
      (if (Variables|Default|GetisOverlapping)
        (Variables|/Game/Dynamic/Blueprints/BP_PlayerCamera.BP_PlayerCamera_C|SettargetPos (Variables|Default|GetplayerCamera) (Transformation|GetWorldLocation (Variables|Default|GetCameraTarget)))
        (CallFunction|MoveCameraTargettoPlayerZPos)))))

(fn ConstructionScript)

(fn MoveCameraTargettoPlayerZPos
  (bind _returnvalue (Game|GetPlayerCharacter 0))
  (bind _cameratarget (Variables|Default|GetCameraTarget))
  (bind _returnvalue_2 (Transformation|GetWorldLocation _cameratarget))
  (bind _returnvalue_3 (Transformation|GetActorLocation _returnvalue))
  (if (not (== (.z _returnvalue_2) (.z _returnvalue_3)))
    (LocalVariables|SetcameraX (.x _returnvalue_2))
    (LocalVariables|SetcameraY (.y _returnvalue_2))
    (LocalVariables|SetplayerZ (.z _returnvalue_3))
    (bind _output_get (LocalVariables|Setvector (Math|Vector|MakeVector (LocalVariables|GetcameraX) (LocalVariables|GetcameraY) (LocalVariables|GetplayerZ))))
    (Transformation|SetWorldLocation (Variables|Default|GetCameraTarget) _output_get false false)))
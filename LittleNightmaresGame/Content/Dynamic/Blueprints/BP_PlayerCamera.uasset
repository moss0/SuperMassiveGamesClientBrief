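; BP_PlayerCamera is a camera actor that becomes the first player's view target on BeginPlay and turns to face the player character.
; Each Tick, CameraState selects either an instant look-at rotation or a smoothed one interpolated at RotateInterpSpeed.
; The live graph changes only rotation; nodes for setting transform and location and for interpolating position are left unconnected.
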(event EventBeginPlay
  (Game|Player|SetViewTargetwithBlend (Game|GetPlayerController 0) self 0.0 "VTBlend_Linear" 0.0 false))

(event EventTick
  (params (DeltaSeconds :type Float%20%28single-precision%29))
  (Variables|Default|SetDelta%20Seconds DeltaSeconds)
  (switch Utilities|FlowControl|Switch|SwitchonEnum_PlayerCameraModes (Variables|Default|GetcameraState)
    (:NewEnumerator1
      (Transformation|SetActorRotation (Math|Rotator|FindLookatRotation (Transformation|GetActorLocation) (Transformation|GetActorLocation (Game|GetPlayerCharacter 0)))))
    (:NewEnumerator0
      (Transformation|SetActorRotation (Math|Interpolation|RInterpTo (.rotation (Transformation|GetActorTransform)) (Math|Rotator|FindLookatRotation (Transformation|GetActorLocation) (Transformation|GetActorLocation (Game|GetPlayerCharacter 0))) (Variables|Default|GetDelta%20Seconds) (Variables|Default|GetrotateInterpSpeed))))))

(fn ConstructionScript)